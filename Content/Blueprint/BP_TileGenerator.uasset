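; Procedural tile-layout actor that fills a set width and length with box tiles and grout, optionally rebuilding in the construction script.
; It merges offset tile boxes into one mesh section, staggering alternate rows for a zigzag pattern, and adds a grout slab as a second section.
; Edge tiles are cut by clamping vertices, with UVs derived from clamped positions, or dropped in whole-tile mode, which shrinks the covered area.
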(fn `UserConstructionScript`
  (if (`self.자동 업데이트 사용`)
    (`self.타일 생성하기`)))

(fn `타일 생성하기`
  (locals (`가로 FirstIndex` :type Integer))
  (bind _proceduralmesh (`self.ProceduralMesh`))
  (bind _generatedarea_box (`self.GeneratedArea Box`))
  (bind `_시공면적_폭_width_` (`self.시공면적 폭(Width)`))
  (bind `_시공면적_길이_length_` (`self.시공면적 길이(Length)`))
  (bind _proceduralmesh_2 (`self.ProceduralMesh`))
  (bind _returnvalue (* (`self.시공면적 폭(Width)`) 0.5))
  (bind _returnvalue_2 (* (`self.시공면적 길이(Length)`) 0.5))
  (bind _returnvalue_3 (+ (`self.타일 가로`) (`self.가로 메지`)))
  (bind _returnvalue_4 (+ (`self.타일 세로`) (`self.세로 메지`)))
  (bind _returnvalue_5 (`KismetMathLibrary.FTrunc` (/ (+ `_시공면적_폭_width_` (`self.가로 오프셋`) (`self.지그재그 간격`)) _returnvalue_3)))
  (bind _returnvalue_6 (`KismetMathLibrary.FTrunc` (/ (+ `_시공면적_길이_length_` (`self.세로 오프셋`)) _returnvalue_4)))
  (`|ExecutionSequence`
    (:`then_0`
      (`BoxComponent.SetBoxExtent` _generatedarea_box (`KismetMathLibrary.MakeVector` _returnvalue _returnvalue_2 10.0) true)
      (`SceneComponent.K2_SetRelativeLocation` _generatedarea_box (`KismetMathLibrary.MakeVector` _returnvalue _returnvalue_2) false false)
      (set `self.가로 타일 자름` (mod `_시공면적_폭_width_` _returnvalue_3))
      (set `self.세로 타일 자름` (mod `_시공면적_길이_length_` _returnvalue_4))
      (if (`self.온장만 (자름 없이)`)
        (bind _output_get (set `self.가로 타일 개수` _returnvalue_5))
        (bind _output_get_2 (set `self.세로 타일 개수` _returnvalue_6))
        (set `self.시공 결과 폭` (* _output_get (+ (`self.타일 가로`) (`self.가로 메지`))))
        (set `self.시공 결과 길이` (* _output_get_2 (+ (`self.타일 세로`) (`self.세로 메지`))))
        (else
          (set `self.가로 타일 개수` (+ _returnvalue_5 1))
          (set `self.세로 타일 개수` (+ _returnvalue_6 1))
          (set `self.시공 결과 폭` (`self.시공면적 폭(Width)`))
          (set `self.시공 결과 길이` (`self.시공면적 길이(Length)`)))))
    (:`then_1`
      (`KismetArrayLibrary.Array_Clear` (`self.Vertices`))
      (`KismetArrayLibrary.Array_Clear` (`self.Triangles`))
      (`KismetArrayLibrary.Array_Clear` (`self.UVs`))
      (`KismetArrayLibrary.Array_Clear` (`self.Normals`))
      (`KismetArrayLibrary.Array_Clear` (`self.Tangents`)))
    (:`then_2`
      (for _index (range (`self.세로 타일 개수`))
        (`|ExecutionSequence`
          (:`then_0`
            (`/Engine/EditorBlueprintResources/StandardMacros.FlipFlop`
              (:`A`
                (set `self.지그재그 오프셋` (`self.지그재그 간격`))
                (if (and (> (`self.지그재그 간격`) 0.0) (`self.온장만 (자름 없이)`))
                  (set `local.가로 FirstIndex` 1)))
              (:`B`
                (set `self.지그재그 오프셋` 0.0)
                (set `local.가로 FirstIndex` 0))))
          (:`then_1`
            (for _index_2 (range (`local.가로 FirstIndex`) (`self.가로 타일 개수`))
              (bind (_vertices _triangles _normals _uvs _tangents) (`KismetProceduralMeshLibrary.GenerateBoxMesh` (`KismetMathLibrary.MakeVector` (* (`self.타일 가로`) 0.5) (* (`self.타일 세로`) 0.5) (* (`self.타일 두께`) 0.5))))
              (for _array_element _triangles
                (`KismetArrayLibrary.Array_Add` (`self.Triangles`) (+ _array_element (`KismetArrayLibrary.Array_Length` (`self.Vertices`)))))
              (`KismetArrayLibrary.Array_Append` (`self.Normals`) _normals)
              (`KismetArrayLibrary.Array_Append` (`self.Tangents`) _tangents)
              (for _array_element_2 _vertices
                (bind (_returnvalue_x _returnvalue_y _returnvalue_z) (`KismetMathLibrary.BreakVector` (+ _array_element_2 (`KismetMathLibrary.MakeVector` (+ (* _index_2 (+ (`self.타일 가로`) (`self.가로 메지`))) (- (* (`self.타일 가로`) 0.5) (+ (`self.가로 오프셋`) (`self.지그재그 오프셋`)))) (+ (* _index (+ (`self.타일 세로`) (`self.세로 메지`))) (- (* (`self.타일 세로`) 0.5) (`self.세로 오프셋`)))))))
                (bind _returnvalue_7 (`KismetMathLibrary.FClamp` _returnvalue_x 0.0 (`self.시공 결과 폭`)))
                (bind _returnvalue_8 (`KismetMathLibrary.FClamp` _returnvalue_y 0.0 (`self.시공 결과 길이`)))
                (`KismetArrayLibrary.Array_Add` (`self.Vertices`) (`KismetMathLibrary.MakeVector` _returnvalue_7 _returnvalue_8 _returnvalue_z))
                (`KismetArrayLibrary.Array_Add` (`self.UVs`) (`KismetMathLibrary.MakeVector2D` (/ (+ _returnvalue_7 (`self.가로 오프셋`)) (+ (`self.타일 가로`) (`self.가로 메지`))) (/ (+ _returnvalue_8 (`self.세로 오프셋`)) (+ (`self.타일 세로`) (`self.세로 메지`)))))))))))
    (:`then_3`
      (`ProceduralMeshComponent.CreateMeshSection_LinearColor` :`self` _proceduralmesh :`Vertices` (`self.Vertices`) :`Triangles` (`self.Triangles`) :`Normals` (`self.Normals`) :`UV0` (`self.UVs`) :`Tangents` (`self.Tangents`) :`bCreateCollision` true)
      (`PrimitiveComponent.SetMaterial` _proceduralmesh 0 (`self.타일 머티리얼`))
      (bind (_vertices_2 _triangles_2 _normals_2 _uvs_2 _tangents_2) (`KismetProceduralMeshLibrary.GenerateBoxMesh` (`KismetMathLibrary.MakeVector` (* (+ (`self.시공 결과 폭`) (`self.가로 메지`)) 0.5) (* (+ (`self.시공 결과 길이`) (`self.세로 메지`)) 0.5) (* (`self.메지 두께`) 0.5))))
      (for (_array_element_3 _array_index) _vertices_2
        (`KismetArrayLibrary.Array_Set` _vertices_2 _array_index (+ _array_element_3 (`KismetMathLibrary.MakeVector` (* (- (`self.시공 결과 폭`) (`self.가로 메지`)) 0.5) (* (- (`self.시공 결과 길이`) (`self.세로 메지`)) 0.5))))
        (`ProceduralMeshComponent.CreateMeshSection_LinearColor` :`self` _proceduralmesh_2 :`SectionIndex` 1 :`Vertices` _vertices_2 :`Triangles` _triangles_2 :`Normals` _normals_2 :`UV0` _uvs_2 :`Tangents` _tangents_2 :`bCreateCollision` true :!label _label)
        (`PrimitiveComponent.SetMaterial` _proceduralmesh_2 1 (`self.메지 머티리얼`)))
      (goto _label))
    (:`then_4`
      (set `self.타일 개수` (* (`self.가로 타일 개수`) (`self.세로 타일 개수`))))))