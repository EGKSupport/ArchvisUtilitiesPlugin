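; Architectural massing study actor that rebuilds a schematic building and its area summary in the construction script.
; Child BoxComponents become procedural sections, either full height or slab thickness.
; Their areas are summed by component tags into a TextRender showing square metres, pyeong and floor area ratio, excluding "service" from totals.
; Optionally, two sunlight-setback planes tilted by north offsets slice the mass, copying cut-off halves into separate cutout-material meshes.
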(fn `UserConstructionScript`
  (locals (`Room반복자` :type Integer) (`RoomVertex반복자` :type Integer) (NewLocalVar_0 :type "Rotator Structure" :default (struct)) (NewLocalVar_1 :type "Vector Structure" :default (0.0 0.0 0.0)))
  (`self.가설계 업데이트`))

(fn `가설계 업데이트`
  (locals (`층별면적Key` :type String))
  (bind `_가로_일조사선` (`self.가로 일조사선`))
  (bind `_세로_일조사선` (`self.세로 일조사선`))
  (bind `_층별_연면적map` (`self.층별 연면적Map`))
  (bind `_층별_연면적map_2` (`self.층별 연면적Map`))
  (bind `_용적율_산정면적` (`self.용적율 산정면적`))
  (bind `_층별면적key` (`local.층별면적Key`))
  (bind (_returnvalue_x _returnvalue_y) (`KismetMathLibrary.BreakVector` (`BoxComponent.GetScaledBoxExtent` `_가로_일조사선`)))
  (bind _returnvalue_x_2 (`KismetMathLibrary.BreakVector` (`BoxComponent.GetScaledBoxExtent` `_세로_일조사선`)))
  (bind _output_get (set `self.용적율 산정면적` 0.0))
  (set `self.건축 연면적` _output_get)
  (`BlueprintMapLibrary.Map_Clear` (`self.층별 연면적Map`))
  (set `self.건축개요 문자열` "")
  (`ProceduralMeshComponent.ClearAllMeshSections` (`self.ProceduralMesh1`))
  (`ProceduralMeshComponent.ClearAllMeshSections` (`self.ProceduralMesh2`))
  (`|ExecutionSequence`
    (:`then_0`
      (`SceneComponent.K2_SetRelativeLocationAndRotation` `_가로_일조사선` (`KismetMathLibrary.MakeVector` 0.0 (* _returnvalue_y -1.0)) (`KismetMathLibrary.MakeRotator` 0.0 (`KismetMathLibrary.DegAtan2` (/ 2.0 (`KismetMathLibrary.DegSin` (`self.가로 NorthOffset`))) 1.0)) false false)
      (`SceneComponent.K2_SetRelativeLocationAndRotation` `_세로_일조사선` (`KismetMathLibrary.MakeVector` _returnvalue_x_2) (`KismetMathLibrary.MakeRotator` (`KismetMathLibrary.DegAtan2` (/ 2.0 (`KismetMathLibrary.DegSin` (`self.세로 NorthOffset`))) 1.0)) false false))
    (:`then_1`
      (for (_array_element _array_index) (`SceneComponent.GetChildrenComponents` (`self.ProceduralMesh`) true)
        (bind _asbox_collision (cast `BoxComponent` _array_element))
        (bind (_returnvalue_x_3 _returnvalue_y_2 _returnvalue_z) (`KismetMathLibrary.BreakVector` (`BoxComponent.GetScaledBoxExtent` _asbox_collision)))
        (bind _returnvalue (`KismetMathLibrary.SelectFloat` _returnvalue_z (`self.슬라브 두께`) (`self.벽 채움`)))
        (bind (_vertices _triangles _normals _uvs _tangents) (`KismetProceduralMeshLibrary.GenerateBoxMesh` (`KismetMathLibrary.MakeVector` _returnvalue_x_3 _returnvalue_y_2 _returnvalue)))
        (`|ExecutionSequence`
          (:`then_0`
            (for (_array_element_2 _array_index_2) _vertices
              (`|ExecutionSequence`
                (:`then_0`
                  (bind (_returnvalue_x_4 _returnvalue_y_3 _returnvalue_z_2) (`KismetMathLibrary.BreakVector` (`BoxComponent.GetScaledBoxExtent` _asbox_collision)))
                  (`KismetArrayLibrary.Array_Set` _vertices _array_index_2 (+ (`SceneComponent.RelativeLocation` _asbox_collision) _array_element_2 (`KismetMathLibrary.MakeVector` 0.0 0.0 (+ _returnvalue (* _returnvalue_z_2 -1.0))))))
                (:`then_1`
                  (`ProceduralMeshComponent.CreateMeshSection_LinearColor` :`self` (`self.ProceduralMesh`) :`SectionIndex` _array_index :`Vertices` _vertices :`Triangles` _triangles :`Normals` _normals :`UV0` _uvs :`Tangents` _tangents)
                  (`PrimitiveComponent.SetMaterial` (`self.ProceduralMesh`) _array_index (`self.M_Box`))))))
          (:`then_1`
            (for _array_element_3 (`ActorComponent.ComponentTags` _asbox_collision)
              (set `local.층별면적Key` (`KismetStringLibrary.Concat_StrStr` (`local.층별면적Key`) " " (`KismetStringLibrary.Conv_NameToString` _array_element_3))))
            (`BlueprintMapLibrary.Map_Add` `_층별_연면적map_2` `_층별면적key` (+ (* _returnvalue_x_3 _returnvalue_y_2 0.0004) (`BlueprintMapLibrary.Map_Find` `_층별_연면적map_2` `_층별면적key`)))
            (set `local.층별면적Key` "")))))
    (:`then_2`
      (for _array_element_4 (`SceneComponent.GetChildrenComponents` (`self.ProceduralMesh`) true)
        _))
    (:`then_3`
      (bind _keys (`BlueprintMapLibrary.Map_Keys` `_층별_연면적map`))
      (for (_array_element_5 _array_index_3) _keys
        (bind _values (`BlueprintMapLibrary.Map_Values` `_층별_연면적map`))
        (bind _output (`|GetArrayItem` _values _array_index_3))
        (set `self.건축개요 문자열` (`KismetStringLibrary.Concat_StrStr` (`self.건축개요 문자열`) _array_element_5 " : " (`KismetTextLibrary.Conv_TextToString` (`KismetTextLibrary.Conv_DoubleToText` _output "HalfToEven" false true 1 324 0 1)) " (" (`KismetTextLibrary.Conv_TextToString` (`KismetTextLibrary.Conv_DoubleToText` (/ _output 3.3) "HalfToEven" false true 1 324 0 1)) "py) \n"))
        (set `self.건축 연면적` (+ _output (`self.건축 연면적`)))
        (if (`KismetStringLibrary.NotEqual_StrStr` _array_element_5 "service")
          (set `self.용적율 산정면적` (+ _output (`self.용적율 산정면적`)))))
      (set `self.건축개요 문자열` (`KismetStringLibrary.Concat_StrStr` (`self.건축개요 문자열`) "" " Total Floor Area : " (`KismetTextLibrary.Conv_TextToString` (`KismetTextLibrary.Conv_DoubleToText` `_용적율_산정면적` "HalfToEven" false true 1 324 0 1)) " (" (`KismetTextLibrary.Conv_TextToString` (`KismetTextLibrary.Conv_DoubleToText` (/ `_용적율_산정면적` 3.3) "HalfToEven" false true 1 324 0 1)) "py) \n"))
      (set `self.용적율` (* (/ (`self.용적율 산정면적`) (`self.대지면적`)) 100.0))
      (set `self.건축개요 문자열` (`KismetStringLibrary.Concat_StrStr` (`self.건축개요 문자열`) "" " Floor Area Ratio : " (`KismetTextLibrary.Conv_TextToString` (`KismetTextLibrary.Conv_DoubleToText` (`self.용적율`) "HalfToEven" false true 1 324 0 1)) "%"))
      (`TextRenderComponent.K2_SetText` (`self.TextRender`) (`KismetTextLibrary.Conv_StringToText` (`self.건축개요 문자열`))))
    (:`then_4`
      (if (`self.일조사선 자동체크`)
        (`self.일조사선 자름`)))))

(fn `일조사선 자름`
  (bind _proceduralmesh1 (`self.ProceduralMesh1`))
  (bind `_세로_일조사선` (`self.세로 일조사선`))
  (bind `_가로_일조사선` (`self.가로 일조사선`))
  (`|ExecutionSequence`
    (:`then_0`
      (bind _outotherhalfprocmesh (`KismetProceduralMeshLibrary.SliceProceduralMesh` (`self.ProceduralMesh`) (`SceneComponent.K2_GetComponentLocation` `_세로_일조사선`) (* (`SceneComponent.GetUpVector` `_세로_일조사선`) -1.0) true "NoCap"))
      (`|ExecutionSequence`
        (:`then_0`
          (`SceneComponent.K2_SetWorldLocation` _proceduralmesh1 (`SceneComponent.K2_GetComponentLocation` _outotherhalfprocmesh) false false)
          (bind (_vertices _triangles _normals _uvs _tangents) (`KismetProceduralMeshLibrary.GetSectionFromProceduralMesh` _outotherhalfprocmesh))
          (`ProceduralMeshComponent.CreateMeshSection_LinearColor` :`self` _proceduralmesh1 :`Vertices` _vertices :`Triangles` _triangles :`Normals` _normals :`UV0` _uvs :`Tangents` _tangents)
          (`ProceduralMeshComponent.CreateMeshSection_LinearColor` :`self` (`self.ProceduralMesh1`) :`Vertices` _vertices :`Triangles` _triangles :`Normals` _normals :`UV0` _uvs :`Tangents` _tangents)
          (`PrimitiveComponent.SetMaterial` (`self.ProceduralMesh1`) 0 (`self.M_Cutout`)))
        (:`then_1`
          (`SceneComponent.K2_DetachFromComponent` _outotherhalfprocmesh "KeepRelative" "KeepRelative" "KeepRelative" true)
          (`ActorComponent.K2_DestroyComponent` _outotherhalfprocmesh))))
    (:`then_1`
      (bind _outotherhalfprocmesh_2 (`KismetProceduralMeshLibrary.SliceProceduralMesh` (`self.ProceduralMesh`) (`SceneComponent.K2_GetComponentLocation` `_가로_일조사선`) (`KismetMathLibrary.Normal` (* (`SceneComponent.GetUpVector` `_가로_일조사선`) -1.0)) true "NoCap"))
      (`|ExecutionSequence`
        (:`then_0`
          (`SceneComponent.K2_SetWorldLocation` (`self.ProceduralMesh2`) (`SceneComponent.K2_GetComponentLocation` _outotherhalfprocmesh_2) false false)
          (bind (_vertices_2 _triangles_2 _normals_2 _uvs_2 _tangents_2) (`KismetProceduralMeshLibrary.GetSectionFromProceduralMesh` _outotherhalfprocmesh_2))
          (`ProceduralMeshComponent.CreateMeshSection_LinearColor` :`self` (`self.ProceduralMesh2`) :`Vertices` _vertices_2 :`Triangles` _triangles_2 :`Normals` _normals_2 :`UV0` _uvs_2 :`Tangents` _tangents_2)
          (`PrimitiveComponent.SetMaterial` (`self.ProceduralMesh2`) 0 (`self.M_Cutout`)))
        (:`then_1`
          (`SceneComponent.K2_DetachFromComponent` _outotherhalfprocmesh_2 "KeepRelative" "KeepRelative" "KeepRelative" true)
          (`ActorComponent.K2_DestroyComponent` _outotherhalfprocmesh_2))))))